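; Actor component that keeps a character's weapon inventory and equips weapons onto the player.
; InitalizeInventory caches the owning Character, and StoreWeapon adds weapons to the Inventory array without duplicates.
; EquipWeapon initializes a WeaponBase with that character and attaches it to the GripPoint socket on the PlayerM_CH Arms.
; HideWeapon is an empty stub, and the integer weapon parameter is unused throughout.
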(fn `Equip Weapon`
  (params (Weapon :type "Actor Object Reference") (`Weapon Int 0` :type Integer))
  (returns (`Success?` :type Boolean))
  (bind _character (`self.Character`))
  (bind _asweapon_base (cast `/Game/Blueprints/Weapons/Actors/WeaponBase` Weapon))
  (`/Game/Blueprints/misc/WeaponInterface.Initalize Weapon` _asweapon_base _character)
  (bind _asplayer_m_ch (cast `/Game/Blueprints/Player/Main/PlayerM_CH` _character))
  (`Actor.K2_AttachToComponent` _asweapon_base (`/Game/Blueprints/Player/Main/PlayerM_CH.Arms` _asplayer_m_ch) "GripPoint" "KeepRelative" "KeepRelative" "KeepRelative" true)
  (return false))

(fn `Hide Weapon`
  (params (Weapon :type "Actor Object Reference") (`Weapon Int 0` :type Integer))
  (returns (`Success?` :type Boolean))
  (return false))

(fn `Initalize Inventory`
  (params (Character :type "Character Object Reference"))
  (returns (`Success?` :type Boolean))
  (set `self.Character` Character)
  (return false))

(fn `Store Weapon`
  (params (Weapon :type "Actor Object Reference") (`Weapon Int 0` :type Integer))
  (returns (`Success?` :type Boolean))
  (`KismetArrayLibrary.Array_AddUnique` (`self.Inventory`) Weapon)
  (return false))